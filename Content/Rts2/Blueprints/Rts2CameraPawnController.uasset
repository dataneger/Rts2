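; Player controller for an RTS game that drives the camera pawn and handles building placement.
; Axis input and screen-edge checks move the pawn at zoom-scaled or fixed speeds respectively, while gated mouse input rotates it and zoom actions adjust spring arm length.
; On begin play it spawns a construction manager and ghost building and creates the HUD.
; In build mode the ghost follows the cursor; left click queues construction.
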(event `self.ReceiveBeginPlay`
  (bind _returnvalue (`KismetMathLibrary.MakeTransform` (0.0 0.0 0.0)))
  ;[1 1 1] Begin Play
  (`|ExecutionSequence`
    (:`then_0`
      (`self.ReferenceCasts`))
    (:`then_1`
      (bind _returnvalue_2 (`|SpawnActorFromClass` "/Game/Rts2/Blueprints/Construction/ConstructionManager_BP.ConstructionManager_BP_C" _returnvalue "AlwaysSpawn" "OverrideRootScale" null null))
      (set `self.ConstructManagerRef` _returnvalue_2))
    (:`then_2`
      (bind _returnvalue_3 (`|SpawnActorFromClass` "/Game/Rts2/Blueprints/Buildings/GhostBuilding_BP.GhostBuilding_BP_C" _returnvalue "AlwaysSpawn" "OverrideRootScale" null self null))
      (set `self.GhostBuildingRef` _returnvalue_3))
    (:`then_3`
      (`WidgetBlueprintLibrary.SetInputMode_GameAndUIEx` self null "LockAlways")
      (`self.CreateHuds`)
      (`UserWidget.AddToViewport` (`self.MainHudRef`) 0))))

(event `InputAxis|MoveForward`
  (params (AxisValue :type "Float (single-precision)"))
  ;[1 1 1] Camera Controll
  ;;[1 1 1] Movement X
  (if (not (`self.DisableCamNav`))
    (`self.K2_SetActorTransform` (`self.Rts2CameraPawnRef`) (`self.MovementX` (`self.MovementSpeedCalculation`) (`self.FastMoveMultiplier`) AxisValue (`self.Rts2CameraPawnRef`)) false false)))

(event `InputAxisKey|MouseX`
  (params (AxisValue :type "Float (single-precision)"))
  ;[1 1 1] Camera Controll
  ;;[1 1 1] Edge Movement
  (if (not (`self.DisableCamNav`))
    (bind (_deltayspeed _deltaxspeed) (`self.ScreenEdgeMovement` :!label _label))
    (`self.K2_AddActorLocalOffset` (`self.Rts2CameraPawnRef`) (`KismetMathLibrary.MakeVector` _deltaxspeed _deltayspeed) true false)))

(event `InputAxis|MoveRight`
  (params (AxisValue :type "Float (single-precision)"))
  ;[1 1 1] Camera Controll
  ;;[1 1 1] Movement Y
  (if (not (`self.DisableCamNav`))
    (`self.K2_SetActorTransform` (`self.Rts2CameraPawnRef`) (`KismetMathLibrary.MakeTransform` (`KismetMathLibrary.MakeVector` (.x (.location (`self.MovementY` AxisValue (`self.MovementSpeedCalculation`) (`self.FastMoveMultiplier`) (`self.Rts2CameraPawnRef`)))) (.y (.location (`self.MovementY` AxisValue (`self.MovementSpeedCalculation`) (`self.FastMoveMultiplier`) (`self.Rts2CameraPawnRef`)))) 100.0) (.rotation (`self.MovementY` AxisValue (`self.MovementSpeedCalculation`) (`self.FastMoveMultiplier`) (`self.Rts2CameraPawnRef`))) (.scale (`self.MovementY` AxisValue (`self.MovementSpeedCalculation`) (`self.FastMoveMultiplier`) (`self.Rts2CameraPawnRef`)))) false false)))

(event `InputAxisKey|MouseY`
  (params (AxisValue :type "Float (single-precision)"))
  ;[1 1 1] Camera Controll
  ;;[1 1 1] Edge Movement
  (if (not (`self.DisableCamNav`))
    (goto _label :!via `MouseY`)))

(event `Key|LeftShift`
  (params (Key :type "Key Structure"))
  ;[1 1 1] Camera Controll
  ;;[1 1 1] Speed multiplier
  (:`Pressed`
    (set `self.FastMoveMultiplier` 2.0))
  (:`Released`
    (set `self.FastMoveMultiplier` 1.0)))

(event `InputAxisKey|MouseX`
  (params (AxisValue :type "Float (single-precision)"))
  ;[1 1 1] Camera Controll
  ;;[1 1 1] Pan X
  (`/Engine/EditorBlueprintResources/StandardMacros.Gate` true :!label _label_2
    (:`Exit`
      (`self.K2_SetActorRotation` (`self.Rts2CameraPawnRef`) (`KismetMathLibrary.MakeRotator` (.roll (`self.K2_GetActorRotation` (`self.Rts2CameraPawnRef`))) (.pitch (`self.K2_GetActorRotation` (`self.Rts2CameraPawnRef`))) (+ (.yaw (`self.K2_GetActorRotation` (`self.Rts2CameraPawnRef`))) (* (`self.PanSensitivity`) AxisValue))) false))))

(event `InputAction|Pan`
  (params (Key :type "Key Structure"))
  ;[1 1 1] Camera Controll
  ;;[1 1 1] Pan X
  (:`Pressed`
    (set `self.DisableCamNav` true)
    (goto _label_2 :!via `Open`))
  (:`Released`
    (set `self.DisableCamNav` false)
    (goto _label_2 :!via `Close`)))

(event `InputAction|ZoomIn`
  (params (Key :type "Key Structure"))
  (bind _springarm (`/Game/Rts2/Blueprints/Rts2CameraPawn.SpringArm` (`self.Rts2CameraPawnRef`)))
  ;[1 1 1] Camera Controll
  ;;[1 1 1] Camera Zoom
  (:`Pressed`
    (set `SpringArmComponent.TargetArmLength` (`KismetMathLibrary.FClamp` (- (`SpringArmComponent.TargetArmLength` _springarm) (`self.ZoomSensitivity`)) 500.0 (`self.MaxArmDistance`)) _springarm)))

(event `InputAxisKey|MouseY`
  (params (AxisValue :type "Float (single-precision)"))
  ;[1 1 1] Camera Controll
  ;;[1 1 1] Pan Y
  (`/Engine/EditorBlueprintResources/StandardMacros.Gate` true :!label _label_3
    (:`Exit`
      (`self.K2_SetActorRotation` (`self.Rts2CameraPawnRef`) (`KismetMathLibrary.MakeRotator` (.roll (`self.K2_GetActorRotation` (`self.Rts2CameraPawnRef`))) (`KismetMathLibrary.FClamp` (+ (.pitch (`self.K2_GetActorRotation` (`self.Rts2CameraPawnRef`))) (* (`self.PanSensitivity`) AxisValue)) -15.0 45.0) (.yaw (`self.K2_GetActorRotation` (`self.Rts2CameraPawnRef`)))) false))))

(event `InputAction|ZoomOut`
  (params (Key :type "Key Structure"))
  (bind _springarm (`/Game/Rts2/Blueprints/Rts2CameraPawn.SpringArm` (`self.Rts2CameraPawnRef`)))
  ;[1 1 1] Camera Controll
  ;;[1 1 1] Camera Zoom
  (:`Pressed`
    (set `SpringArmComponent.TargetArmLength` (`KismetMathLibrary.FClamp` (+ (`self.ZoomSensitivity`) (`SpringArmComponent.TargetArmLength` _springarm)) 500.0 (`self.MaxArmDistance`)) _springarm)))

(event `InputAction|Pan`
  (params (Key :type "Key Structure"))
  ;[1 1 1] Camera Controll
  ;;[1 1 1] Pan Y
  (:`Pressed`
    (set `self.DisableCamNav` true)
    (goto _label_3 :!via `Open`))
  (:`Released`
    (set `self.DisableCamNav` false)
    (goto _label_3 :!via `Close`)))

(event `InputAction|ZoomReset`
  (params (Key :type "Key Structure"))
  ;[1 1 1] Camera Controll
  ;;[1 1 1] Reset Camera Zoom
  (:`Pressed`
    (set `SpringArmComponent.TargetArmLength` 1500.0 (`/Game/Rts2/Blueprints/Rts2CameraPawn.SpringArm` (`self.Rts2CameraPawnRef`)))))

(event `InputAction|PanReset`
  (params (Key :type "Key Structure"))
  (bind _rts2camerapawnref (`self.Rts2CameraPawnRef`))
  ;[1 1 1] Camera Controll
  ;;[1 1 1] Pan reset
  (:`Pressed`
    (`self.K2_SetActorRotation` _rts2camerapawnref (`KismetMathLibrary.MakeRotator` (.roll (`self.K2_GetActorRotation` _rts2camerapawnref)) 0.0 (.yaw (`self.K2_GetActorRotation` _rts2camerapawnref))) false)))

(event `Key|LeftMouseButton`
  (params (Key :type "Key Structure"))
  (:`Pressed`
    (if (`self.BuildModeActive`)
      (bind _constructionstruct (`/Game/Rts2/Blueprints/Buildings/GhostBuilding_BP.GetConstructionStruct` (`self.GhostBuildingRef`)))
      (`/Game/Rts2/Blueprints/Construction/ConstructionManager_BP.QueueConstruction` (`self.ConstructManagerRef`) _constructionstruct)
      (`/Game/Rts2/Blueprints/Buildings/GhostBuilding_BP.KillGhost` (`self.GhostBuildingRef`)))))

(event `self.ReceiveTick`
  (params (DeltaSeconds :type "Float (single-precision)"))
  ;[1 1 1] Building constructions
  ;;[1 1 1] Trace mouse
  (if (`self.BuildModeActive`)
    (if (!= (`self.GhostBuildingRef`) null)
      (`/Game/Rts2/Blueprints/Buildings/GhostBuilding_BP.SetCursorPosition` (`self.GhostBuildingRef`) (`/Game/Rts2/Libraries/FunctionLibrary.Set Cursor World Position` self (`self.SetSightDistance`))))))

(event `InputAction|Deselect`
  (params (Key :type "Key Structure"))
  ;[1 1 1] Building constructions
  ;;[1 1 1] Cancel building
  (:`Pressed`
    (if (`self.BuildModeActive`)
      (`/Game/Rts2/Blueprints/Buildings/GhostBuilding_BP.KillGhost` (`self.GhostBuildingRef`))
      (set `self.BuildModeActive` false))))

(fn `MovementSpeedCalculation`
  (returns (MoveSensitivity :type "Float (double-precision)"))
  (return (`KismetMathLibrary.FClamp` (/ (`SpringArmComponent.TargetArmLength` (`/Game/Rts2/Blueprints/Rts2CameraPawn.SpringArm` (`self.Rts2CameraPawnRef`))) 100.0) 5.0 20.0)))

(fn `SetCalendar`
  (params (Date :type "Array of Integer (by ref)"))
  (returns (Success :type Boolean))
  (return false))

(fn `SetClock`
  (params (Time :type "Array of Integer (by ref)"))
  (returns (Success :type Boolean))
  (return false))

(fn `SetSightDistance`
  (returns (SightDistance :type "Float (double-precision)"))
  (return (+ (`self.SightDistance`) (`SpringArmComponent.TargetArmLength` (`/Game/Rts2/Blueprints/Rts2CameraPawn.SpringArm` (`self.Rts2CameraPawnRef`))))))

(fn `UserConstructionScript`)